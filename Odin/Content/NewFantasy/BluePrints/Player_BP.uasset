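; Player character for a fantasy RPG, handling camera-relative movement, combat, HP/MP, death and HUD interactions.
; Attack inputs fill damage or debuff structs and open a gated in-battle timer that expires without renewed combat.
; While the attack window is open, Tick overlaps a weapon-socket sphere, hits each enemy once and applies effects through GameMode.
; Keys drive pickup, NPC talk, toolbar items, a shop and saving, while a SceneCapture renders the character for equipment UI.
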(event Custom|ReceiveMPBuff
  (params (addMP :type Integer))
  ;[1 1 1] Update MP By Buff
  (Variables|状态|Setm_currentMagic (Math|Integer|Clamp(Integer) (+ (Variables|状态|Getm_currentMagic) addMP) 0 (Variables|Attribute|Getm_maxMagic)))
  (Default|UpdatePlayerMPInfo (Variables|/Game/NewFantasy/GameSetting/Fantasy_HUD.Fantasy_HUD_C|GetPlayingUI (Variables|Instance|GethudInstance)) (Variables|Attribute|Getm_maxMagic) (Variables|状态|Getm_currentMagic)))

(event Custom|SkillAttack
  (params (SkillType :type PlayerBattleState%20Enum :default "NewEnumerator2"))
  ;[1 1 1] SkillAttack
  (CallFunction|ClearSkillStruct)
  (if (Variables|状态|GetIsInBattle)
    _
    (else
      (CallFunction|StartBattle)))
  (Variables|状态|SetBattleState SkillType)
  (Variables|状态|SetcanNotMove false)
  (Variables|Battle|SetcurrentDebuff_Damage_Struct (Utilities|Select :Index SkillType :NewEnumerator2 "" :NewEnumerator0 "" :NewEnumerator1 "" :NewEnumerator3 (Utilities|Struct|MakeDebuff_Damage_Struct "灼烧" (* (Variables|Attribute|Getm_attackPower) 0.1) 8.0 2.0 "/Game/NewFantasy/Assets/UIAssets/Skill_Icon/spell-7.spell-7" true) :NewEnumerator4 "" :NewEnumerator5 "" :NewEnumerator6 "")))

(event Custom|StartBattle
  ;[1 1 1] 战斗开始
  (Variables|状态|SetState "NewEnumerator0")
  (Variables|状态|SetIsInBattle true)
  (Variables|状态|SetinBattleTimer 0.0)
  ;[1 1 1] 战斗计时
  (Utilities|FlowControl|Gate true) ; enters at Open
)

(event Custom|ReceiveHPBuff
  (params (addHP :type Integer))
  ;[1 1 1] Update HP By Buff
  (bind _output_get (Variables|状态|Setm_currentLife (Math|Integer|Clamp(Integer) (+ (Variables|状态|Getm_currentLife) addHP) 0 (Variables|Attribute|Getm_maxLife))))
  (Default|UpdatePlayerHPInfo (Variables|/Game/NewFantasy/GameSetting/Fantasy_HUD.Fantasy_HUD_C|GetPlayingUI (Variables|Instance|GethudInstance)) (Variables|Attribute|Getm_maxLife) _output_get))

(event Custom|StartRenderCharactor
  (bind _scenecapturecomponent2d (Variables|Default|GetSceneCaptureComponent2D))
  ;[1 1 1] 装备栏捕捉角色renderTarget
  (Variables|/Script/Engine.SceneCaptureComponent|SetShowOnlyActors _scenecapturecomponent2d (Utilities|Array|MakeArray self))
  (Components|Activation|SetActive _scenecapturecomponent2d true false))

(event Custom|ClearSkillStruct
  ;[1 1 1] Clear Skill Struct
  (Variables|Battle|SetcurrentImmediateAttack_Struct "")
  (Variables|Battle|SetcurrentDebuff_Damage_Struct "")
  (Variables|Battle|SetcurrentDebuff_State_Struct ""))

(event Custom|EndRenderCharactor
  ;[1 1 1] 装备栏捕捉角色renderTarget
  (Components|Activation|SetActive (Variables|Default|GetSceneCaptureComponent2D) false false))

(event EventBeginPlay
  (bind _m_maxlife (Variables|Attribute|Getm_maxLife))
  (bind _m_maxmagic (Variables|Attribute|Getm_maxMagic))
  (bind _output_get (Variables|Cache|Setm_playerController (Game|GetPlayerController 0)))
  ;[1 1 1] 鼠标mouse over
  (Variables|/Script/Engine.PlayerController|SetbEnableMouseOverEvents _output_get true)
  ;[1 1 1] Hud
  (bind _asfantasy_hud (Utilities|Casting|CastToFantasy_HUD (HUD|GetHUD (Game|GetPlayerController 0))))
  (Variables|Instance|SethudInstance _asfantasy_hud)
  ;[1 1 1] GameMode Instance
  (bind _asfantasy_game_mode (Utilities|Casting|CastToFantasyGameMode (Game|GetGameMode)))
  (Variables|Instance|SetgameMode _asfantasy_game_mode)
  ;[1 1 1] 玩家数据记录中心
  (bind _asfantasy_player_state (Utilities|Casting|CastToFantasyPlayerState (Variables|GetPlayerState)))
  (Variables|Default|SetmyPlayer_State _asfantasy_player_state)
  (Utilities|FlowControl|Delay 0.5)
  ;[1 1 1] 更新基础和装备属性到玩家属性‘
  (Default|UpdateArmoBagAttributetoPlayer (Variables|Instance|GethudInstance))
  (bind _output_get_2 (Variables|状态|Setm_currentLife _m_maxlife))
  (bind _output_get_3 (Variables|状态|Setm_currentMagic _m_maxmagic))
  (Default|UpdatePlayerHPInfo (Variables|/Game/NewFantasy/GameSetting/Fantasy_HUD.Fantasy_HUD_C|GetPlayingUI (Variables|Instance|GethudInstance)) _m_maxlife _output_get_2)
  (Default|UpdatePlayerMPInfo (Variables|/Game/NewFantasy/GameSetting/Fantasy_HUD.Fantasy_HUD_C|GetPlayingUI (Variables|Instance|GethudInstance)) _m_maxmagic _output_get_3))

(event Collision|EventActorBeginOverlap
  (params (OtherActor :type Actor%20Object%20Reference)))

(event EventTick
  (params (DeltaSeconds :type Float%20%28single-precision%29))
  (bind _m_currentmovespeed (Variables|Attribute|Getm_currentMoveSpeed))
  (bind _m_maxmovespeed (Variables|Attribute|Getm_maxMoveSpeed))
  (bind _isaccelerate (Variables|状态|GetisAccelerate))
  (bind _returnvalue (Math|Float|SelectFloat _m_currentmovespeed _m_maxmovespeed _isaccelerate))
  (Utilities|FlowControl|Sequence
    (:then_0
      ;[1 1 1] 摄像机旋转
      (Pawn|Input|AddControllerYawInput (Input|AxisValues|GetTurn)) ; Z轴旋转
      (Pawn|Input|AddControllerPitchInput (Input|AxisValues|GetLookUp)) ; Y轴旋转
    )
    (:then_1
      ;[1 1 1] 移动
      (if (not (or (Variables|状态|GetcanNotMove) (or (Variables|状态|GetisDeath) (Variables|状态|GetAttackPointCollisionEnabled))))
        (bind _output_get (Variables|Cache|SetcurrentMoveVector (* (Math|Vector|Normalize (* (Math|Vector|Normalize (Math|Vector|MakeVector (Input|AxisValues|GetMoveForward) (Input|AxisValues|GetMoveRight) 0.0)) (Math|Float|SelectFloat (Variables|Attribute|Getm_currentMoveSpeed) (Variables|Attribute|Getm_maxMoveSpeed) (Variables|状态|GetisAccelerate)))) _returnvalue)))
        (if (> (Math|Vector|VectorLength _output_get) 0.0)
          ;;[1 1 1] 走动速度
          (Variables|状态|SetState "NewEnumerator3")
          (Variables|/Script/Engine.CharacterMovementComponent|SetMaxWalkSpeed (Variables|Character|GetCharacterMovement) _returnvalue)
          (Pawn|Input|AddMovementInput (Math|Transform|TransformDirection (Transformation|GetActorTransform) (* _output_get DeltaSeconds)) 1.0 false)
          (Transformation|SetActorRotation (Math|Rotator|Lerp(Rotator) (Transformation|GetActorRotation) (Math|Rotator|MakeRotator 0.0 0.0 (.Yaw (Math|Rotator|BreakRotator (Pawn|GetControlRotation :!class /Script/Engine.Pawn)))) (* (Utilities|Time|GetWorldDeltaSeconds) (Variables|Attribute|Getm_rotateSpeed)) true)))))
    (:then_2
      ;[1 1 1] 战斗计时
      (Utilities|FlowControl|Gate true :!label _label
        (:Exit
          (bind _output_get_2 (Variables|状态|SetinBattleTimer (+ (Variables|状态|GetinBattleTimer) (Utilities|Time|GetWorldDeltaSeconds))))
          (if (> _output_get_2 6.0)
            (Variables|状态|SetIsInBattle false)
            (Variables|状态|SetinBattleTimer 0.0)
            (goto _label Close)))))
    (:then_3
      ;[1 1 1] 攻击判定
      (Utilities|AttackCollision))))

(event Game|Damage|EventAnyDamage
  (params (Damage :type Float%20%28single-precision%29) (DamageType :type Damage%20Type%20Object%20Reference) (InstigatedBy :type Controller%20Object%20Reference) (DamageCauser :type Actor%20Object%20Reference))
  ;[1 1 1] ReceiveDamage
  (if (>= (Variables|状态|Getm_currentLife) 0)
    (Variables|状态|Setm_currentLife (Math|Integer|Clamp(Integer) (- (Variables|状态|Getm_currentLife) (Math|Float|Truncate Damage)) 0 (Variables|Attribute|Getm_maxLife)))
    (CallFunction|StartBattle)
    (Default|CallPlayerHPChangeDisPatcher (Variables|Attribute|Getm_maxLife) (Variables|状态|Getm_currentLife))
    (if (== (Variables|状态|Getm_currentLife) 0)
      (Components|Activation|Deactivate (Variables|Character|GetCharacterMovement))
      (Variables|状态|SetisDeath true)
      (Default|CallPlayerDeathDisPatcher)
      (Variables|状态|SetState "NewEnumerator4"))))

(event Input|ActionEvents|InputActionJump
  (params (Key :type Key%20Structure))
  ;[1 1 1] 跳
  (:Pressed
    (Character|Jump)
    (Variables|状态|SetState "NewEnumerator2"))
  (:Released
    (Variables|状态|SetState "NewEnumerator1")))

(event Input|ActionEvents|InputActionPlayerNormalAttack
  (params (Key :type Key%20Structure))
  ;[1 1 1] NormalAttack
  (:Pressed
    (CallFunction|ClearSkillStruct)
    (if (Variables|状态|GetIsInBattle)
      _
      (else
        (CallFunction|StartBattle)))
    (Variables|状态|SetBattleState "NewEnumerator1")
    (Variables|状态|SetcanNotMove false)
    (Variables|Battle|SetcurrentImmediateAttack_Struct (Utilities|Struct|MakeImmediateAttack_Struct "普通攻击" (Math|Conversions|ToFloat(Integer) (Variables|Attribute|Getm_attackPower)) (Variables|Attribute|GetmBaoJi)))))

(event Input|KeyboardEvents|L
  (params (Key :type Key%20Structure))
  (:Pressed
    (bind _asfantasy_game_instance (Utilities|Casting|CastToFantasy_GameInstance (Game|GetGameInstance)))
    (bind _savesuccess (Default|SaveGameData _asfantasy_game_instance))
    (Development|PrintString (select _savesuccess "Save Success" "Save Fail"))))

(event Input|KeyboardEvents|F
  (params (Key :type Key%20Structure))
  (bind _hudinstance (Variables|Instance|GethudInstance))
  ;[1 1 1] 交互按键 PickUp Item / 对话
  (:Pressed
    (Utilities|FlowControl|Sequence
      (:then_0
        (Default|PickUponMouseOverEnemy _hudinstance))
      (:then_1
        (Default|NPCTalk _hudinstance)))))

(event Input|KeyboardEvents|2
  (params (Key :type Key%20Structure))
  (:Pressed
    (CallFunction|UseToolBagItem 1)))

(event Input|KeyboardEvents|3
  (params (Key :type Key%20Structure))
  (:Pressed
    (CallFunction|UseToolBagItem 2)))

(event Input|KeyboardEvents|4
  (params (Key :type Key%20Structure))
  (:Pressed
    (CallFunction|UseToolBagItem 3)))

(event Input|KeyboardEvents|5
  (params (Key :type Key%20Structure))
  (:Pressed
    (CallFunction|UseToolBagItem 4)))

(event Input|KeyboardEvents|6
  (params (Key :type Key%20Structure))
  (:Pressed
    (CallFunction|UseToolBagItem 5)))

(event Input|KeyboardEvents|7
  (params (Key :type Key%20Structure))
  (:Pressed
    (CallFunction|UseToolBagItem 6)))

(event Input|KeyboardEvents|LeftShift
  (params (Key :type Key%20Structure))
  (bind _state (Variables|状态|GetState))
  ;[1 1 1] 跑/走
  (:Pressed
    (switch Utilities|FlowControl|Switch|SwitchonPlayerStateEnum _state
      (:NewEnumerator3
        (Variables|状态|SetisAccelerate true))))
  (:Released
    (switch Utilities|FlowControl|Switch|SwitchonPlayerStateEnum _state
      (:NewEnumerator3
        (Variables|状态|SetisAccelerate false)))))

(event Input|KeyboardEvents|I
  (params (Key :type Key%20Structure))
  ;[1 1 1] 显示商品列表
  (:Pressed
    (Default|ToggleShopWidget (Variables|/Game/NewFantasy/GameSetting/Fantasy_HUD.Fantasy_HUD_C|GetPlayingUI (Variables|Instance|GethudInstance)) (Utilities|Array|MakeArray (Utilities|Struct|MakeShopGood_Struct "砍木斧" 1) (Utilities|Struct|MakeShopGood_Struct "小瓶红药" 3)) 0 false false)))

(event Input|KeyboardEvents|Delete
  (params (Key :type Key%20Structure))
  ;[1 1 1] 删除快捷item
  (:Pressed
    (Default|DeleteToolItem (Variables|Instance|GethudInstance))))

(event Input|KeyboardEvents|Backspace
  (params (Key :type Key%20Structure))
  ;[1 1 1] 删除快捷item
  (:Pressed
    (Default|DeleteToolItem (Variables|Instance|GethudInstance))))

(event Input|KeyboardEvents|G
  (params (Key :type Key%20Structure)))

(event Input|KeyboardEvents|8
  (params (Key :type Key%20Structure))
  (:Pressed
    (CallFunction|UseToolBagItem 7)))

(fn ConstructionScript)

(fn GetAliveEnemyArrayinRange
  (params (attackRange :type Float%20%28single-precision%29) (reverseResult :type Boolean))
  (bind _outactors (Actor|GetAllActorsOfClass "/Game/NewFantasy/BluePrints/EnemyBase_BP.EnemyBase_BP_C"))
  (for _array_element _outactors
    (if (not reverseResult)
      (if (and (not (Variables|/Game/NewFantasy/BluePrints/EnemyBase_BP.EnemyBase_BP_C|GetisDeath _array_element)) (< (Transformation|GetDistanceTo _array_element) attackRange))
        (Utilities|Array|Add (LocalVariables|GettempEnemyArray) _array_element :!label _label))
      (elif (or (Variables|/Game/NewFantasy/BluePrints/EnemyBase_BP.EnemyBase_BP_C|GetisDeath _array_element) (> (Transformation|GetDistanceTo _array_element) attackRange))
        (goto _label))))
  (return (LocalVariables|GettempEnemyArray)))

(fn UseToolBagItem
  (params (index :type Integer))
  (bind _values (Utilities|Map|Values (Variables|/Game/NewFantasy/UI/Bag.Bag_C|GetBagBGItemArray (Variables|/Game/NewFantasy/GameSetting/Fantasy_HUD.Fantasy_HUD_C|GettoolBag (Variables|Instance|GethudInstance)))))
  (if (Utilities|IsValid (Variables|/Game/NewFantasy/UI/BagBG_Item.BagBG_Item_C|GetfilledItem (Utilities|Array|Get(acopy) _values index)))
    (Default|UseItem (Variables|/Game/NewFantasy/UI/BagBG_Item.BagBG_Item_C|GetfilledItem (Utilities|Array|Get(acopy) _values index)))
    (else
      (Development|PrintString "No Item"))))

(fn GetDieEnemyforPickUpItem
  (bind _outactors (Actor|GetAllActorsOfClass "/Script/AIModule.AIController"))
  (for _array_element _outactors
    (bind _asenemy_base_bp (Utilities|Casting|CastToEnemyBase_BP (Pawn|GetControlledPawn _array_element)))))