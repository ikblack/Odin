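; Base NPC for a fantasy RPG, handling talk, shop and quest giving.
; Talk opens a multi-option menu or floating text; dialogue walks DataTable rows by index and can load quests to accept or turn in.
; Player-state quest status drives the overhead icon.
; Two detection spheres control distance-based head-widget scaling on Tick, and close dialogue and shop when the player leaves, rewinding dialogue to its saved checkpoint.
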(event OnComponentBeginOverlap(DetectPlayerSphereCollision)
  (params (OverlappedComponent :type Primitive%20Component%20Object%20Reference) (OtherActor :type Actor%20Object%20Reference) (OtherComp :type Primitive%20Component%20Object%20Reference) (OtherBodyIndex :type Integer) (bFromSweep :type Boolean) (SweepResult :type Hit%20Result%20Structure%20%28by%20ref%29))
  ;[1 1 1] 玩家进入或离开视野
  (Utilities|Casting|CastToPlayer_BP OtherActor)
  (Variables|Default|SetisUpdateUIScale true))

(event OnComponentEndOverlap(DetectPlayerSphereCollision)
  (params (OverlappedComponent :type Primitive%20Component%20Object%20Reference) (OtherActor :type Actor%20Object%20Reference) (OtherComp :type Primitive%20Component%20Object%20Reference) (OtherBodyIndex :type Integer))
  ;[1 1 1] 玩家进入或离开视野
  (Utilities|Casting|CastToPlayer_BP OtherActor)
  (Variables|Default|SetisUpdateUIScale false))

(event OnComponentBeginOverlap(DialogDetectSphereCollision)
  (params (OverlappedComponent :type Primitive%20Component%20Object%20Reference) (OtherActor :type Actor%20Object%20Reference) (OtherComp :type Primitive%20Component%20Object%20Reference) (OtherBodyIndex :type Integer) (bFromSweep :type Boolean) (SweepResult :type Hit%20Result%20Structure%20%28by%20ref%29))
  ;[1 1 1] 对话框显示/消失距离
)

(event OnComponentEndOverlap(DialogDetectSphereCollision)
  (params (OverlappedComponent :type Primitive%20Component%20Object%20Reference) (OtherActor :type Actor%20Object%20Reference) (OtherComp :type Primitive%20Component%20Object%20Reference) (OtherBodyIndex :type Integer))
  (bind _hudinstance (Variables|Default|GethudInstance))
  (bind _dialog_ui (Variables|Default|Getdialog_UI))
  (bind _playingui (Variables|/Game/NewFantasy/GameSetting/Fantasy_HUD.Fantasy_HUD_C|GetPlayingUI _hudinstance))
  ;[1 1 1] 对话框显示/消失距离
  (Utilities|Casting|CastToPlayer_BP OtherActor)
  (Default|CallOnPlayerOutOfTaskDialogRange)
  (Utilities|FlowControl|Sequence
    (:then_0
      (if (== (Variables|/Game/NewFantasy/UI/Dialog_UI.Dialog_UI_C|GetcurrentDialogOwner _dialog_ui) self)
        (Default|CloseDialogUI _dialog_ui)))
    (:then_1
      (if (== (Variables|/Game/NewFantasy/UI/ShopWidget.ShopWidget_C|GetShopNPC_Owner (Variables|/Game/NewFantasy/UI/PlayingUI.PlayingUI_C|GetShopWidget _playingui)) self)
        (Default|ToggleShopWidget _playingui (Variables|Default|GetshopGoodsArray) 0 true false)))
    (:then_2
      (CallFunction|ResetBreakDialogprocess))))

(event Custom|Task
  ;[1 1 1] 开始对话
  (bind _taskstate (CallFunction|GetTaskState))
  (switch Utilities|FlowControl|Switch|SwitchonTaskState _taskstate
    (:NewEnumerator6
      _)
    (:NewEnumerator0
      _)
    (:NewEnumerator2
      _))
  (Default|SetTaskContentWindow (Variables|Default|GethudInstance) (Utilities|Array|Get(acopy) (Variables|Default|GetTaskArray)) _taskstate self)
  (Utilities|FlowControl|Delay 0.2)
  (EventDispatchers|BindEventtoButtonClick (Variables|Default|Getdialog_UI) (delegate Custom|TaskConfirmButtonClick)))

(event Custom|Talk
  (bind _多功能条目 (Variables|Default|Get多功能条目))
  (bind _多功能数量 (Variables|Default|Get多功能数量))
  ;[1 1 1] 玩家和NPC交互的开始
  (if (> _多功能数量 0)
    (bind _dialog_ui (Default|SetDialogUIText (Variables|Default|GethudInstance) true (Utilities|String|ToString(Name) (Variables|Default|GetNPCName)) (Variables|Default|GetNPC多功能对话显示内容) _多功能数量 (Utilities|Array|Get(acopy) _多功能条目) (Utilities|Array|Get(acopy) _多功能条目 1) (select (== _多功能数量 3) (Utilities|Array|Get(acopy) _多功能条目 2) "") self (Variables|Default|GetDefaultHeadImage)))
    (EventDispatchers|BindEventtoButtonClick _dialog_ui (delegate Custom|DecideDoWhat))
    (else
      ;[1 1 1] 开始对话
      ;;[1 1 1] 浮动窗口对话
      (Default|SetDialogWindowText (Variables|Default|GethudInstance) self (.Description (Utilities|Struct|BreakDialogAssets_DataTable (Variables|Default|GetcurrentDialog_Data))) 5.0))))

(event Custom|DialogConfirmed
  (params (ButtonIndex :type Integer))
  (bind _currentdialog_data (Variables|Default|GetcurrentDialog_Data))
  (bind (_nextistask _nexttaskname) (Utilities|Struct|BreakDialogAssets_DataTable _currentdialog_data))
  ;[1 1 1] 对话按钮绑定事件
  (if _nextistask
    (switch int ButtonIndex
      (:1
        (if (not (Utilities|Name|Equal(Name) _nexttaskname "None"))
          (CallFunction|LoadTaskData _nexttaskname)
          (CallFunction|Task)
          (CallFunction|GetNextDialogData false false)))
      (:2
        (Default|CloseDialogUI (Variables|Default|Getdialog_UI) :!label _label)
        (CallFunction|ResetBreakDialogprocess))
      (:3
        (goto _label)))
    (else
      (CallFunction|GetNextDialogData true false))))

(event Custom|GetNextDialogData
  (params (GoToNextDialog :type Boolean) (FinishTask :type Boolean))
  (bind _currentdialog_data (Variables|Default|GetcurrentDialog_Data))
  (bind _nextdialogindex (Utilities|Struct|BreakDialogAssets_DataTable _currentdialog_data))
  ;[1 1 1] 获得下一个对话资料
  (if FinishTask
    (Math|Integer|IncrementInt (Variables|Default|GetcurrentDialogIndex)
      (:%20%20
        (bind _addsuccess (CallFunction|SetCurrentDialogData :!label _label))
        (if _addsuccess
          (if GoToNextDialog
            (CallFunction|TaskDialog))
          (else
            (Default|CloseDialogUI (Variables|Default|Getdialog_UI) :!label _label_2)))))
    (elif (== _nextdialogindex (Variables|Default|GetcurrentDialogIndex))
      (goto _label_2)
      (else
        (Variables|Default|SetcurrentDialogIndex _nextdialogindex)
        (goto _label)))))

(event Custom|TaskDialog
  (bind _currentdialog_data (Variables|Default|GetcurrentDialog_Data))
  (bind (_nextistask _nexttaskname _nextdialogindex _description _headiconpath) (Utilities|Struct|BreakDialogAssets_DataTable _currentdialog_data))
  ;[1 1 1] 检查任务完成情况
  (if (> (Utilities|Array|Length (Variables|Default|GetTaskArray)) 0)
    (bind _taskstate (CallFunction|GetTaskState))
    (if (Utilities|Select :Index _taskstate :NewEnumerator6 false :NewEnumerator0 false :NewEnumerator1 false :NewEnumerator2 true :NewEnumerator3 false :NewEnumerator5 false :NewEnumerator4 false)
      (CallFunction|Task)
      (else
        ;[1 1 1] 开始对话
        ;;[1 1 1] 浮动窗口对话
        (Default|SetDialogUIText (Variables|Default|GethudInstance) true (Utilities|String|ToString(Name) (Variables|Default|GetNPCName)) _description (select _nextistask 2 1) "接受" "拒绝" "关闭" self _headiconpath :!label _label)
        (Utilities|FlowControl|Delay 0.2)
        (CallFunction|BindDialogConfirmEvent)))
    (else
      (goto _label))))

(event Custom|TaskConfirmButtonClick
  (params (ButtonIndex :type Integer))
  ;[1 1 1] 开始对话
  (Utilities|FlowControl|Sequence
    (:then_0
      (switch Utilities|FlowControl|Switch|SwitchonTaskState (stale Custom|Task _taskstate)
        (:NewEnumerator0
          (switch int ButtonIndex
            (:1
              (Default|AddNewTasktoPlayerData (Variables|/Game/NewFantasy/BluePrints/Player_BP.Player_BP_C|GetmyPlayer_State (Variables|/Game/NewFantasy/GameSetting/Fantasy_HUD.Fantasy_HUD_C|GetPlayer_BP (Variables|Default|GethudInstance))) (Utilities|Array|Get(acopy) (Variables|Default|GetTaskArray)))
              (CallFunction|GetNextDialogData true false)
              (Variables|Default|SetNewStartDialogProcessIndex (Variables|Default|GetcurrentDialogIndex) :!label _label)
              (CallFunction|UpdateTaskIcon))
            (:2
              (CallFunction|ResetBreakDialogprocess :!label _label_2))
            (:3
              (goto _label_2))))
        (:NewEnumerator2
          (bind _finishsuccess (Default|FinishTaskGetAward (Variables|/Game/NewFantasy/GameSetting/Fantasy_HUD.Fantasy_HUD_C|Getdialog_UI (Variables|Default|GethudInstance))))
          (if _finishsuccess
            (Utilities|Array|RemoveIndex (Variables|Default|GetTaskArray))
            (CallFunction|GetNextDialogData true true)
            (goto _label)))))
    (:then_1
      (Default|CloseDialogUI (Variables|Default|Getdialog_UI))
      (CallFunction|GetNextDialogData false false))))

(event Custom|BindDialogConfirmEvent
  ;[1 1 1] 对话按钮绑定事件
  (EventDispatchers|BindEventtoButtonClick (Variables|Default|Getdialog_UI) (delegate Custom|DialogConfirmed)))

(event Custom|DecideDoWhat
  (params (ButtonIndex :type Integer))
  ;[1 1 1] 玩家和NPC交互的开始
  (switch int ButtonIndex
    (:1
      (CallFunction|Shop))
    (:2
      (CallFunction|TaskDialog))
    (:3
      ;[1 1 1] 开始对话
      ;;[1 1 1] 浮动窗口对话
      (Default|SetDialogWindowText (Variables|Default|GethudInstance) self (.Description (Utilities|Struct|BreakDialogAssets_DataTable (Variables|Default|GetcurrentDialog_Data))) 5.0))))

(event Custom|Shop
  (Default|ToggleShopWidget (Variables|/Game/NewFantasy/GameSetting/Fantasy_HUD.Fantasy_HUD_C|GetPlayingUI (Variables|Default|GethudInstance)) (Variables|Default|GetshopGoodsArray) self true true)
  (Default|CloseDialogUI (Variables|Default|Getdialog_UI)))

(event Custom|ResetBreakDialogprocess
  ;[1 1 1] 重置因为中途打断的对话进度
  (Variables|Default|SetcurrentDialogIndex (Variables|Default|GetNewStartDialogProcessIndex))
  (CallFunction|SetCurrentDialogData))

(event EventBeginPlay
  (bind _maxhp (Variables|Default|GetMaxHP))
  ;[1 1 1] 缓存头部UI组件
  (bind _asnpc_head_widget (Utilities|Casting|CastToNPC_Head_Widget (UserInterface|GetUserWidgetObject (Variables|Default|GetTaskWidget))))
  (bind _output_get (Variables|Default|SetHPBarWidget _asnpc_head_widget))
  (Default|SetHPBarOwnerName (Variables|/Game/NewFantasy/UI/NPC_Head_Widget.NPC_Head_Widget_C|GetHPBar _output_get) (Utilities|Text|FormatText "{0} 等级：{1}" (Utilities|Text|ToText(Name) (Variables|Default|GetNPCName)) (Variables|Default|Getlevel)))
  (bind _output_get_2 (Variables|Default|SetcurrentHP _maxhp))
  (Default|UpdateHP (Variables|/Game/NewFantasy/UI/NPC_Head_Widget.NPC_Head_Widget_C|GetHPBar _output_get) _output_get_2 _maxhp)
  ;[1 1 1] 等待主要实例初始化
  (Utilities|FlowControl|Delay 0.5)
  (Utilities|FlowControl|Sequence
    (:then_0
      ;[1 1 1] 缓存Hud 和 dialog UI
      (bind _asfantasy_hud (Utilities|Casting|CastToFantasy_HUD (HUD|GetHUD (Game|GetPlayerController 0))))
      (bind _output_get_3 (Variables|Default|SethudInstance _asfantasy_hud))
      (Variables|Default|Setdialog_UI (Variables|/Game/NewFantasy/GameSetting/Fantasy_HUD.Fantasy_HUD_C|Getdialog_UI _output_get_3))
      (CallFunction|SetCurrentDialogData))
    (:then_1
      ;[1 1 1] 针对玩家出生就在碰撞范围内的情况,没有进入碰撞反应,同时初始化任务图标
      (|DoOnceMultiInput
        (:A%20Out
          (Variables|Default|SetisUpdateUIScale true)
          (CallFunction|UpdateTaskIcon)
          (Utilities|FlowControl|Delay 0.1)
          (Variables|Default|SetisUpdateUIScale (< (Transformation|GetDistanceTo (Game|Player|GetPlayerPawn 0) self) (Class|SphereComponent|GetUnscaledSphereRadius (Variables|Default|GetDetectPlayerSphereCollision))))
          (EventDispatchers|BindEventtoOnTaskCompelete (Variables|Default|GethudInstance) (EventDispatchers|CreateEvent :!event ListenTaskFinish)))))))

(event Collision|EventActorBeginOverlap
  (params (OtherActor :type Actor%20Object%20Reference)))

(event EventTick
  (params (DeltaSeconds :type Float%20%28single-precision%29))
  (bind _returnvalue (Game|GetPlayerController 0))
  (bind _taskwidget (Variables|Default|GetTaskWidget))
  (bind _detectplayerspherecollision (Variables|Default|GetDetectPlayerSphereCollision))
  (bind _hpbarwidget (Variables|Default|GetHPBarWidget))
  (bind _returnvalue_2 (Class|SphereComponent|GetUnscaledSphereRadius _detectplayerspherecollision))
  (bind _returnvalue_3 (Transformation|GetWorldLocation _taskwidget))
  (bind _outlocation (Actor|GetActorEyesViewPoint _returnvalue))
  (bind _returnvalue_4 (- _returnvalue_3 _outlocation))
  (bind _returnvalue_5 (Math|Vector|VectorLength _returnvalue_4))
  (bind _returnvalue_6 (Math|Float|MapRangeUnclamped _returnvalue_5 3e+02 _returnvalue_2 1.0 0.5))
  (bind _returnvalue_7 (Math|Vector2D|MakeVector2D _returnvalue_6 _returnvalue_6))
  ;[1 1 1] Update
  ;[1 1 1] 缩放血条
  (if (Variables|Default|GetisUpdateUIScale)
    (bind _output_get (Variables|Default|SetHP_scaleVecotor2 _returnvalue_7))
    (if (not (< (.X (Math|Vector2D|BreakVector2D _output_get)) 0.5))
      (Widget|SetVisibility _hpbarwidget "Visible")
      (Widget|Transform|SetRenderScale _hpbarwidget _returnvalue_7)
      (Class|CanvasPanelSlot|SetPosition (Class|WidgetLayoutLibrary|SlotasCanvasSlot (Variables|/Game/NewFantasy/UI/NPC_Head_Widget.NPC_Head_Widget_C|GetContainer _hpbarwidget)) (Math|Vector2D|MakeVector2D -212.960938 (Math|Float|MapRangeUnclamped (.X (Math|Vector2D|BreakVector2D _output_get)) 1.0 0.5 -2.5e+02 0.0)))
      (else
        (Widget|SetVisibility _hpbarwidget "Hidden")))))

(event MouseInput|EventActorBeginCursorOver
  ;[1 1 1] 鼠标mouse over  触发谈话 提示
  (Variables|/Game/NewFantasy/GameSetting/Fantasy_HUD.Fantasy_HUD_C|SetcurrentMouseOverNPC (Variables|Default|GethudInstance) self))

(event MouseInput|EventActorEndCursorOver
  ;[1 1 1] 鼠标mouse over  触发谈话 提示
  (Variables|/Game/NewFantasy/GameSetting/Fantasy_HUD.Fantasy_HUD_C|SetcurrentMouseOverNPC (Variables|Default|GethudInstance) 0))

(fn ConstructionScript)

(fn UpdateTaskIcon
  (bind _taskarray (Variables|Default|GetTaskArray))
  (bind _hpbarwidget (Variables|Default|GetHPBarWidget))
  (bind _image (Variables|/Game/NewFantasy/UI/NPC_Head_Widget.NPC_Head_Widget_C|GetImage _hpbarwidget))
  (bind _brush (Variables|/Script/UMG.Image|GetBrush _image))
  (bind (_imagesize _margin _tintcolor _resourceobject _drawas _tiling _mirroring) (Utilities|Struct|BreakSlateBrush _brush))
  (if (> (Utilities|Array|Length _taskarray) 0)
    (bind _output_get (LocalVariables|SettempTaskname (.TaskName (Utilities|Struct|BreakTask (Utilities|Array|Get(acopy) _taskarray)))))
    ;[1 1 1] 检查玩家数据中的任务状态
    (bind _taskstate (Default|GetTaskState (Variables|/Game/NewFantasy/BluePrints/Player_BP.Player_BP_C|GetmyPlayer_State (Variables|/Game/NewFantasy/GameSetting/Fantasy_HUD.Fantasy_HUD_C|GetPlayer_BP (Variables|Default|GethudInstance))) _output_get))
    (LocalVariables|SettaskState _taskstate)
    (Widget|SetVisibility _image (Utilities|Select :Index (LocalVariables|GettaskState) :NewEnumerator6 "Hidden" :NewEnumerator0 "HitTestInvisible" :NewEnumerator1 "HitTestInvisible" :NewEnumerator2 "HitTestInvisible" :NewEnumerator3 "HitTestInvisible" :NewEnumerator5 "Hidden" :NewEnumerator4 "Hidden"))
    (switch Utilities|FlowControl|Switch|SwitchonTaskState (LocalVariables|GettaskState)
      (:NewEnumerator0
        _)
      (:NewEnumerator1
        _)
      (:NewEnumerator2
        _)
      (:NewEnumerator3
        _))
    (Class|Image|SetBrush _image (Utilities|Struct|MakeSlateBrush "(X=128.000000,Y=128.000000)" _margin _tintcolor (Utilities|Select :Index (LocalVariables|GettaskState) :NewEnumerator6 "/Game/NewFantasy/Assets/UIAssets/黄色叹号.黄色叹号" :NewEnumerator0 "/Game/NewFantasy/Assets/UIAssets/黄色叹号.黄色叹号" :NewEnumerator1 "/Game/NewFantasy/Assets/UIAssets/灰色问号.灰色问号" :NewEnumerator2 "/Game/NewFantasy/Assets/UIAssets/黄色问号.黄色问号" :NewEnumerator3 "/Game/NewFantasy/Assets/UIAssets/灰色叹号.灰色叹号" :NewEnumerator5 0 :NewEnumerator4 0) _drawas _tiling _mirroring))
    (else
      (Widget|SetVisibility (Variables|/Game/NewFantasy/UI/NPC_Head_Widget.NPC_Head_Widget_C|GetImage (Variables|Default|GetHPBarWidget)) "Hidden"))))

(fn SetHeadImageIcon
  (params (visable :type Boolean) (IconTexture :type Texture%202D%20Object%20Reference))
  (bind _hpbarwidget (Variables|Default|GetHPBarWidget))
  (bind _image (Variables|/Game/NewFantasy/UI/NPC_Head_Widget.NPC_Head_Widget_C|GetImage _hpbarwidget))
  (bind _brush (Variables|/Script/UMG.Image|GetBrush _image))
  (bind (_imagesize _margin _tintcolor _resourceobject _drawas _tiling _mirroring) (Utilities|Struct|BreakSlateBrush _brush))
  (Widget|SetVisibility _image (select visable "Collapsed" "HitTestInvisible"))
  (Class|Image|SetBrush _image (Utilities|Struct|MakeSlateBrush "(X=128.000000,Y=128.000000)" _margin _tintcolor IconTexture _drawas _tiling _mirroring)))

(fn FinishTask
  (bind _taskarray (Variables|Default|GetTaskArray))
  (if (> (Utilities|Array|Length _taskarray) 0)
    (Utilities|Array|RemoveIndex _taskarray)
    (CallFunction|UpdateTaskIcon)))

(fn ListenTaskFinish
  (params (TaskName :type Name))
  (bind _taskarray (Variables|Default|GetTaskArray))
  (if (> (Utilities|Array|Length _taskarray) 0)
    (if (Utilities|Name|Equal(Name) (.TaskName (Utilities|Struct|BreakTask (Utilities|Array|Get(acopy) _taskarray))) TaskName)
      (CallFunction|UpdateTaskIcon))))

(fn IsCurrentDialogValid
  (return (Utilities|Enum|Equal(Enum) (.Description (Utilities|Struct|BreakDialogAssets_DataTable (Variables|Default|GetcurrentDialog_Data))) "")))

(fn SetCurrentDialogData
  (bind _currentdialogindex (Variables|Default|GetcurrentDialogIndex))
  (if (> _currentdialogindex 0)
    (bind _returnvalue (Utilities|GetDataTableRow (Variables|Default|GetDialogData) (Utilities|String|StringToName (Utilities|String|ToString(Integer) _currentdialogindex)))
      (:then
        (Variables|Default|SetcurrentDialog_Data _returnvalue)
        (return true)))
    (else
      (return false))))

(fn GetTaskState
  (bind _taskstate (Default|GetTaskState (Variables|/Game/NewFantasy/BluePrints/Player_BP.Player_BP_C|GetmyPlayer_State (Variables|/Game/NewFantasy/GameSetting/Fantasy_HUD.Fantasy_HUD_C|GetPlayer_BP (Variables|Default|GethudInstance))) (.TaskName (Utilities|Struct|BreakTask (Utilities|Array|Get(acopy) (Variables|Default|GetTaskArray))))))
  (return _taskstate))

(fn LoadTaskData
  (params (Taskname :type Name))
  (bind _taskarray (Variables|Default|GetTaskArray))
  (bind _returnvalue (Utilities|GetDataTableRow "/Game/NewFantasy/DataTable/Task.Task" Taskname)
    (:then
      (bind _returnvalue_2 (Utilities|Array|Add _taskarray (Utilities|Struct|MakeTask Taskname "NewEnumerator6" (Utilities|Map|MakeMap "" "") _returnvalue)))
      (Default|SetTaskItemProgressbyRef (Variables|Default|GethudInstance) (Utilities|Array|Get(acopy) _taskarray _returnvalue_2))
      (CallFunction|UpdateTaskIcon))
    (:RowNotFound
      (Development|PrintString (Utilities|String|Append "NPC 未发现任务数据:" (Utilities|String|ToString(Name) Taskname))))))