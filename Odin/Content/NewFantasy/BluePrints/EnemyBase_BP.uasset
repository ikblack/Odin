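; Base enemy character with stats, health, death and loot, whose old Tick combat logic is disconnected in favor of a BehaviorTree.
; A 3D health bar scales with camera distance and receives debuffs.
; Damage starts a timed battle state that binds the attacking player's quest kill event once per fight.
; Death stops the AI brain, collapses the capsule, broadcasts the kill and rolls loot, registered with the HUD for pickup.
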(event OnComponentBeginOverlap(DetectPlayerDistaneCollision)
  (params (OverlappedComponent :type Primitive%20Component%20Object%20Reference) (OtherActor :type Actor%20Object%20Reference) (OtherComp :type Primitive%20Component%20Object%20Reference) (OtherBodyIndex :type Integer) (bFromSweep :type Boolean) (SweepResult :type Hit%20Result%20Structure%20%28by%20ref%29))
  ;[1 1 1] 监测玩家在UI缩放的距离范围内
  (Utilities|Casting|CastToPlayer_BP OtherActor)
  (Variables|Default|SetcanUpdateUIScale true))

(event OnComponentEndOverlap(DetectPlayerDistaneCollision)
  (params (OverlappedComponent :type Primitive%20Component%20Object%20Reference) (OtherActor :type Actor%20Object%20Reference) (OtherComp :type Primitive%20Component%20Object%20Reference) (OtherBodyIndex :type Integer))
  ;[1 1 1] 监测玩家在UI缩放的距离范围内
  (Utilities|Casting|CastToPlayer_BP OtherActor)
  (Variables|Default|SetcanUpdateUIScale false))

(event Custom|OnPlayerDeath
  ;[1 1 1] 战斗逻辑,  不再使用,  改用 BehaviorTree
  ;;[1 1 1] 回到出生点
  (if (not (Variables|Battle|GetisDeath))
    (Utilities|FlowControl|Delay 2.0)
    ;;[1 1 1] 离开出生点2000,而且距离大于500,返回出生位置
    (AI|Navigation|SimpleMovetoLocation (Pawn|GetController) (Variables|临时变量|GetSpawnPosition))
    (Variables|状态|Setstate "NewEnumerator4")
    (Variables|Battle|SetattackTarget 0)
    (Utilities|FlowControl|Delay 2.0 :!label _label)
    (if (< (Math|Vector|VectorLength (- (* (Transformation|GetActorLocation) "1.000000,1.000000,0.000000") (Variables|临时变量|GetSpawnPosition))) 1.5e+02)
      (Variables|状态|Setstate "NewEnumerator0")
      (else
        (goto _label)))))

(event Custom|SpawnedItemPicked
  (params (pickedItem :type Item%20Object%20Reference))
  (bind _spawnedpickupitemarray (Variables|临时变量|GetspawnedPickUpItemArray))
  ;[1 1 1] 拾取敌人单个爆出物体
  (for _array_element _spawnedpickupitemarray
    (if (Utilities|Name|Equal(Name) (.ItemName (Utilities|Struct|BreakPickUpData _array_element)) (.ItemName (Utilities|Struct|BreakItemStruct (Variables|/Game/NewFantasy/UI/Item.Item_C|GetItemStruct_Info pickedItem))))
      (Utilities|Array|RemoveItem _spawnedpickupitemarray _array_element)))
  (if (== (Utilities|Array|Length _spawnedpickupitemarray) 0)
    (CallFunction|PickUpEndItem)))

(event Custom|LeaveBattle
  ;[1 1 1] Battle  战斗状态
  (Variables|Battle|SetInBattle false)
  (Variables|Battle|SetBattleTimeCount 0.0)
  (Utilities|FlowControl|Sequence
    (:then_0
      (bind _asfantasy_player_controller (Utilities|Casting|CastToFantasy_PlayerController (stale Game|Damage|EventAnyDamage InstigatedBy)))
      (Default|UnBindTaskEnemyDieEvent (Variables|/Game/NewFantasy/BluePrints/Fantasy_PlayerController.Fantasy_PlayerController_C|GetmyPlayerState _asfantasy_player_controller) (Variables|Attribute|GetmName) self))
    (:then_1
      (Utilities|FlowControl|DoOnce false) ; enters at Reset
    )))

(event Custom|ReceiveDebuffState
  (params (DebuffBuff :type Debuff%20State%20Struct%20Structure) (DebuffCausor :type Controller%20Object%20Reference) (DeBuffOwner :type Actor%20Object%20Reference))
  ;[1 1 1] 接受DebuffState
  (Default|AddBufforDebuff :self (Variables|Components|GetHpBar) :BuffType "NewEnumerator3" :DebuffState DebuffBuff :BuffName (.DebuffStateName (Utilities|Struct|BreakDebuff_State_Struct DebuffBuff)) :BuffCausor DebuffCausor :BuffOwner DeBuffOwner))

(event Custom|Start/ReStartBattle
  ;[1 1 1] Battle  战斗状态
  (Variables|Battle|SetInBattle true)
  (Variables|Battle|SetBattleTimeCount 0.0))

(event Custom|PickUpItem
  ;[1 1 1] 将爆出的物体发送到拾取背包中  PickUpBag
  (bind _asfantasy_hud (Utilities|Casting|CastToFantasy_HUD (HUD|GetHUD (Game|GetPlayerController 0))))
  (Default|SpawnPickUpItemtoPickUpBag _asfantasy_hud (Variables|临时变量|GetspawnedPickUpItemArray) self))

(event Custom|PickUpEndItem
  (bind _pickupfx (Variables|临时变量|GetpickUpFX))
  ;[1 1 1] 拾取完敌人爆出的物品
  (Utilities|FlowControl|Sequence
    (:then_0
      (if (Utilities|IsValid _pickupfx)
        (Components|DestroyComponent _pickupfx)))
    (:then_1
      (bind _asfantasy_hud (Utilities|Casting|CastToFantasy_HUD (HUD|GetHUD (Game|GetPlayerController 0))))
      (Default|RegisterorUnRegisterPickItemableArray _asfantasy_hud false self))
    (:then_2
      (Variables|状态|SetisPickUped true)
      (Collision|SetCollisionEnabled (Variables|Character|GetMesh) "NoCollision"))))

(event Custom|ReceiveDebuffDamge
  (params (DebuffDamge :type Debuff%20Damage%20Struct%20Structure) (DebuffCausor :type Controller%20Object%20Reference) (DeBuffOwner :type Actor%20Object%20Reference))
  ;[1 1 1] 接受DebuffDamge
  (Default|AddBufforDebuff :self (Variables|Components|GetHpBar) :BuffType "NewEnumerator1" :DebuffDamge DebuffDamge :BuffName (.DebuffDamageName (Utilities|Struct|BreakDebuff_Damage_Struct DebuffDamge)) :BuffCausor DebuffCausor :BuffOwner DeBuffOwner))

(event EventBeginPlay
  (bind _mname (Variables|Attribute|GetmName))
  (bind _returnvalue (Utilities|String|ToString(Name) _mname))
  (Utilities|FlowControl|Sequence
    (:then_0
      (CallFunction|Init)
      (Variables|临时变量|SetSpawnPosition (Transformation|GetActorLocation))
      (Variables|Battle|SetattackCountTime (Variables|Attribute|GetattackInnerTime))
      ;[1 1 1] 初始化生命
      (Variables|Battle|SetmCurrentHP (Variables|Attribute|GetmMaxHP))
      ;[1 1 1] 血条UI信息
      (bind _ashpbar (Utilities|Casting|CastToHPBar (UserInterface|GetUserWidgetObject (Variables|Default|Get3D_UI))))
      (bind _output_get (Variables|Components|SetHpBar _ashpbar))
      (Default|UpdateOwnerNameandLevel _output_get (select (Variables|Attribute|GetIsBoss) (Utilities|String|Append _returnvalue "(BOSS)") _returnvalue) (Utilities|String|ToString(Integer) (Variables|Attribute|GetmLevel)))
      (Default|UpdateHP _output_get (Variables|Battle|GetmCurrentHP) (Variables|Attribute|GetmMaxHP))
      ;[1 1 1] HudInstance
      (bind _asfantasy_hud (Utilities|Casting|CastToFantasy_HUD (HUD|GetHUD (Game|GetPlayerController 0))))
      (bind _output_get_2 (Variables|Instance|SethudInstance _asfantasy_hud))
      ;[1 1 1] 设置HPBar hud instance
      (Variables|/Game/NewFantasy/UI/HPBar.HPBar_C|SethudInstance (Variables|Components|GetHpBar) _output_get_2))
    (:then_1
      ;[1 1 1] 针对玩家出生就在碰撞范围内的情况,没有进入碰撞反应
      (|DoOnceMultiInput
        (:A%20Out
          (Variables|Default|SetcanUpdateUIScale true)
          (Utilities|FlowControl|Delay 0.1)
          (Variables|Default|SetcanUpdateUIScale (< (Transformation|GetDistanceTo (Game|Player|GetPlayerPawn 0) self) (Class|SphereComponent|GetUnscaledSphereRadius (Variables|Default|GetDetectPlayerDistaneCollision)))))))))

(event Game|Damage|EventAnyDamage
  (params (Damage :type Float%20%28single-precision%29) (DamageType :type Damage%20Type%20Object%20Reference) (InstigatedBy :type Controller%20Object%20Reference) (DamageCauser :type Actor%20Object%20Reference))
  (bind _capsulecomponent (Variables|Collision|GetCapsuleComponent))
  ;[1 1 1] Receive Damage
  (if (> (Variables|Battle|GetmCurrentHP) 0)
    ;;[1 1 1] 战斗重置
    (CallFunction|Start/ReStartBattle)
    (Utilities|FlowControl|Sequence
      (:then_0
        (Utilities|FlowControl|DoOnce false
          (:Completed
            (bind _asfantasy_player_controller (Utilities|Casting|CastToFantasy_PlayerController InstigatedBy))
            (Default|BindTaskEnemyDieEvent (Variables|/Game/NewFantasy/BluePrints/Fantasy_PlayerController.Fantasy_PlayerController_C|GetmyPlayerState _asfantasy_player_controller) (Variables|Attribute|GetmName) self))))
      (:then_1
        (Variables|Battle|SetmCurrentHP (Math|Integer|Clamp(Integer) (- (Variables|Battle|GetmCurrentHP) (Math|Float|Truncate Damage)) 0 (Variables|Attribute|GetmMaxHP)))
        (Default|UpdateHP (Variables|Components|GetHpBar) (Variables|Battle|GetmCurrentHP) (Variables|Attribute|GetmMaxHP))
        (if (<= (Variables|Battle|GetmCurrentHP) 0)
          (Variables|Battle|SetisDeath true)
          (Character|StopJumping)
          (Components|Movement|StopMovementImmediately (Variables|Character|GetCharacterMovement))
          (Default|CallOnDeathDispatcher (Variables|Attribute|GetmName) self)
          (CallFunction|OnSelfDie)
          (Variables|/Script/Engine.PrimitiveComponent|SetCanCharacterStepUpOn _capsulecomponent "ECB_Yes")
          (Components|Capsule|SetCapsuleHalfHeight _capsulecomponent 0.0 true)
          (Components|Capsule|SetCapsuleRadius _capsulecomponent 0.0 true)
          (Components|Activation|Deactivate _capsulecomponent))))))

(event EventTick
  (params (DeltaSeconds :type Float%20%28single-precision%29))
  (bind _returnvalue (Game|GetPlayerController 0))
  (bind _hpbar (Variables|Components|GetHpBar))
  (bind _detectplayerdistanecollision (Variables|Default|GetDetectPlayerDistaneCollision))
  (bind _3d_ui (Variables|Default|Get3D_UI))
  (bind _returnvalue_2 (Class|SphereComponent|GetUnscaledSphereRadius _detectplayerdistanecollision))
  (bind _returnvalue_3 (Transformation|GetWorldLocation _3d_ui))
  (bind _outlocation (Actor|GetActorEyesViewPoint _returnvalue))
  (bind _returnvalue_4 (- _returnvalue_3 _outlocation))
  (bind _returnvalue_5 (Math|Vector|VectorLength _returnvalue_4))
  (bind _returnvalue_6 (Math|Float|MapRangeUnclamped _returnvalue_5 3e+02 _returnvalue_2 1.0 0.5))
  (bind _returnvalue_7 (Math|Vector2D|MakeVector2D _returnvalue_6 _returnvalue_6))
  ;[1 1 1] Update
  (Utilities|FlowControl|Sequence
    (:then_0
      ;[1 1 1] 缩放血条
      (if (Variables|Default|GetcanUpdateUIScale)
        (bind _output_get (Variables|临时变量|SetHP_scaleVecotor2 _returnvalue_7))
        (if (not (< (.X (Math|Vector2D|BreakVector2D _output_get)) 0.5))
          (Widget|SetVisibility _hpbar "Visible")
          (Widget|Transform|SetRenderScale _hpbar _returnvalue_7)
          (else
            (Widget|SetVisibility _hpbar "Hidden")))))
    (:then_1
      ;[1 1 1] 战斗计时,6秒无交互,脱离战斗状态
      (if (Variables|Battle|GetInBattle)
        (bind _output_get_2 (Variables|Battle|SetBattleTimeCount (+ (Variables|Battle|GetBattleTimeCount) (Utilities|Time|GetWorldDeltaSeconds))))
        (if (> _output_get_2 6.0)
          (CallFunction|LeaveBattle))))))

(event MouseInput|EventActorBeginCursorOver
  ;[1 1 1] mouse Over
  (if (Variables|状态|GetisPickUped)
    (Variables|临时变量|SetisMouseOver false)
    (else
      (Variables|临时变量|SetisMouseOver true))))

(event MouseInput|EventActorEndCursorOver
  ;[1 1 1] mouse Over
  (Variables|临时变量|SetisMouseOver false))

(fn ConstructionScript)

(fn SetAttribute
  (params (mName :type Name) (IsBoss :type Boolean) (mLevel :type Integer) (mMaxHP :type Integer) (mAttack :type Integer) (mMoveSpeed :type Float%20%28single-precision%29) (mRotateSpeed :type Float%20%28single-precision%29) (mAttackRange :type Float%20%28single-precision%29) (mDefence :type Integer))
  (Utilities|FlowControl|Sequence
    (:then_0
      (Variables|Attribute|SetmName mName))
    (:then_1
      (Variables|Attribute|SetIsBoss IsBoss))
    (:then_2
      (Variables|Attribute|SetmLevel mLevel))
    (:then_3
      (bind _output_get (Variables|Attribute|SetmMaxHP mMaxHP))
      (Variables|Battle|SetmCurrentHP _output_get))
    (:then_4
      (Variables|Attribute|SetmAttack mAttack)
      (Variables|Attribute|SetmDefence mDefence))
    (:then_5
      (bind _output_get_2 (Variables|Attribute|SetmMoveSpeed mMoveSpeed))
      (Variables|/Script/Engine.CharacterMovementComponent|SetMaxWalkSpeed (Variables|Character|GetCharacterMovement) _output_get_2))
    (:then_6
      (Variables|Attribute|SetmRotateSpeed mRotateSpeed))
    (:then_7
      (Variables|Attribute|SetmDetectRange mAttackRange))))

(fn Init
  (return))

(fn RandomIdleState
  (bind _returnvalue (Pawn|GetController))
  (bind _spawnposition (Variables|临时变量|GetSpawnPosition))
  (switch Utilities|FlowControl|Switch|SwitchonEnemyState (Variables|状态|Getstate)
    (:NewEnumerator0
      (if (> (Math|Vector|VectorLength (- (Transformation|GetActorLocation) _spawnposition)) (Variables|Attribute|GetavailableWalkRange))
        ;[1 1 1] Idle活动范围超出可活动范围,返回出生点
        (AI|Navigation|SimpleMovetoLocation _returnvalue _spawnposition)
        (else
          (switch int (Math|Random|RandomInteger 3)
            (:0
              _)
            (:1
              ;[1 1 1] move
              (AI|Navigation|SimpleMovetoLocation _returnvalue (+ (Transformation|GetActorLocation) (* (Transformation|GetActorForwardVector) 3e+02))))
            (:2
              ;[1 1 1] rotate
              (Transformation|AddActorLocalRotation (Math|Rotator|MakeRotator 0.0 0.0 (Math|Random|RandomFloatinRange -1.5e+02 1.5e+02)) false false)))
          (return false))))))

(fn OnSelfDie
  (Utilities|FlowControl|Sequence
    (:then_0
      (Utilities|Casting|CastToPlayer_BP (Game|Player|GetPlayerPawn 0)))
    (:then_1
      (AI|Logic|StopLogic (Variables|/Script/AIModule.AIController|GetBrainComponent (AI|GetAIController self)) "")
      (Variables|Battle|SetInBattle false)
      (Default|HideBaronDeath (Variables|Components|GetHpBar))
      ;[1 1 1] 爆出物体
      (for _array_element (Variables|Attribute|GetpickUpItemArray)
        (if (< (* (Math|Random|RandomFloat) 1e+02) (.Percent (Utilities|Struct|BreakPickUpData _array_element)))
          (Utilities|Array|Add (Variables|临时变量|GetspawnedPickUpItemArray) (Utilities|Struct|MakePickUpData (.ItemName (Utilities|Struct|BreakPickUpData _array_element)) (.Percent (Utilities|Struct|BreakPickUpData _array_element)) (Utilities|Struct|MakeIntVector 0 0 (Math|Random|RandomIntegerinRange (.X (Utilities|Struct|BreakIntVector (.SpawnAmountRange (Utilities|Struct|BreakPickUpData _array_element)))) (.Y (Utilities|Struct|BreakIntVector (.SpawnAmountRange (Utilities|Struct|BreakPickUpData _array_element))))))))))
      (Utilities|FlowControl|Sequence
        (:then_0
          ;;[1 1 1] 有拾取物体生成
          (if (> (Utilities|Array|Length (Variables|临时变量|GetspawnedPickUpItemArray)) 0)
            (Variables|/Script/Engine.PlayerController|SetbEnableMouseOverEvents (Game|GetPlayerController 0) true)
            (bind _asfantasy_hud (Utilities|Casting|CastToFantasy_HUD (HUD|GetHUD (Game|GetPlayerController 0))))
            (Default|RegisterorUnRegisterPickItemableArray _asfantasy_hud true self)))
        (:then_1
          (return false))))))